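; Timed character power-up pickup whose Pickup type selects a speed, jump height, jump count or dash boost, plus its mesh and label.
; Box overlap hides it, then for player-controlled instigators applies Multiplier, waits TimeToEnd, undoes the boost and re-shows it.
; Other overlaps leave it hidden.
; The BP_InteractionTPC cast feeding Player is disconnected, so the IsValid-guarded boosts receive no valid player from this graph.
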(event OnComponentBeginOverlap(Box)
  (params (OverlappedComponent :type Primitive%20Component%20Object%20Reference) (OtherActor :type Actor%20Object%20Reference) (OtherComp :type Primitive%20Component%20Object%20Reference) (OtherBodyIndex :type Integer) (bFromSweep :type Boolean) (SweepResult :type Hit%20Result%20Structure%20%28by%20ref%29))
  (bind _timetoend (Variables|Default|GetTimeToEnd))
  (if (Variables|Default|GetCanPickup)
    (CallFunction|PickedUp)
    (if (Pawn|IsPlayerControlled (Variables|/Script/Engine.Actor|GetInstigator OtherActor))
      (Variables|Default|SetPlayer (stale _asbp_interaction_tpc))
      (switch Utilities|FlowControl|Switch|SwitchonEnum_CharPickups (Variables|Default|GetPickup)
        (:NewEnumerator0
          (CallFunction|SpeedBoost)
          (Utilities|FlowControl|Delay _timetoend)
          (CallFunction|SpeedReset))
        (:NewEnumerator1
          (CallFunction|JumpBoost)
          (Utilities|FlowControl|Delay _timetoend)
          (CallFunction|JumpReset))
        (:NewEnumerator2
          (CallFunction|JumpCountIncreased)
          (Utilities|FlowControl|Delay _timetoend)
          (CallFunction|JumpCountReset))
        (:NewEnumerator3
          (CallFunction|DashIncreased)
          (Utilities|FlowControl|Delay _timetoend)
          (CallFunction|DashReset)))
      (CallFunction|PickupReset))))

(event EventBeginPlay)

(event Collision|EventActorBeginOverlap
  (params (OtherActor :type Actor%20Object%20Reference)))

(event EventTick
  (params (DeltaSeconds :type Float%20%28single-precision%29)))

(fn ConstructionScript
  (Components|StaticMesh|SetStaticMesh (Variables|Default|GetStaticMesh) (Utilities|Select :Index (Variables|Default|GetPickup) :NewEnumerator0 "/Engine/BasicShapes/Cone.Cone" :NewEnumerator1 "/Engine/BasicShapes/Cube.Cube" :NewEnumerator2 "/Engine/EngineMeshes/MaterialSphere.MaterialSphere" :NewEnumerator3 "/Engine/BasicShapes/Cylinder.Cylinder"))
  (Rendering|Components|TextRender|SetText (Variables|Default|GetTextRender) (Utilities|Select :Index (Variables|Default|GetPickup) :NewEnumerator0 (Utilities|Text|MakeLiteralText "Speed Boost") :NewEnumerator1 (Utilities|Text|MakeLiteralText "Jump Boost") :NewEnumerator2 (Utilities|Text|MakeLiteralText "Jump Count") :NewEnumerator3 (Utilities|Text|MakeLiteralText "Dash"))))

(fn SpeedBoost
  (bind _player (Variables|Default|GetPlayer))
  (bind _multiplier (Variables|Default|GetMultiplier))
  (Utilities|IsValid _player
    (:Is%20Valid
      (Variables|/Game/InteractionSystem/ThirdPersonBP/Blueprints/BP_InteractionTPC.BP_InteractionTPC_C|SetWalkSpeed _player (* (Variables|/Game/InteractionSystem/ThirdPersonBP/Blueprints/BP_InteractionTPC.BP_InteractionTPC_C|GetWalkSpeed _player) _multiplier))
      (Variables|/Game/InteractionSystem/ThirdPersonBP/Blueprints/BP_InteractionTPC.BP_InteractionTPC_C|SetRunSpeed _player (* (Variables|/Game/InteractionSystem/ThirdPersonBP/Blueprints/BP_InteractionTPC.BP_InteractionTPC_C|GetRunSpeed _player) _multiplier))
      (Variables|/Script/Engine.CharacterMovementComponent|SetMaxWalkSpeed (Variables|/Script/Engine.Character|GetCharacterMovement _player) (* (Variables|/Game/InteractionSystem/ThirdPersonBP/Blueprints/BP_InteractionTPC.BP_InteractionTPC_C|GetWalkSpeed _player) _multiplier)))))

(fn JumpBoost
  (bind _player (Variables|Default|GetPlayer))
  (bind _charactermovement (Variables|/Script/Engine.Character|GetCharacterMovement _player))
  (Utilities|IsValid _player
    (:Is%20Valid
      (Variables|/Script/Engine.CharacterMovementComponent|SetJumpZVelocity _charactermovement (* (Variables|/Script/Engine.CharacterMovementComponent|GetJumpZVelocity _charactermovement) (Variables|Default|GetMultiplier))))))

(fn JumpCountIncreased
  (bind _player (Variables|Default|GetPlayer))
  (Utilities|IsValid _player
    (:Is%20Valid
      (Variables|/Script/Engine.Character|SetJumpMaxCount _player (+ (Variables|/Script/Engine.Character|GetJumpMaxCount _player) (Math|Float|Truncate (Variables|Default|GetMultiplier)))))))

(fn DashIncreased
  (bind _player (Variables|Default|GetPlayer))
  (Utilities|IsValid _player
    (:Is%20Valid
      (Variables|/Game/InteractionSystem/ThirdPersonBP/Blueprints/BP_InteractionTPC.BP_InteractionTPC_C|SetDashAmount _player (* (Variables|/Game/InteractionSystem/ThirdPersonBP/Blueprints/BP_InteractionTPC.BP_InteractionTPC_C|GetDashAmount _player) (Variables|Default|GetMultiplier))))))

(fn SpeedReset
  (bind _player (Variables|Default|GetPlayer))
  (bind _multiplier (Variables|Default|GetMultiplier))
  (Utilities|IsValid _player
    (:Is%20Valid
      (Variables|/Game/InteractionSystem/ThirdPersonBP/Blueprints/BP_InteractionTPC.BP_InteractionTPC_C|SetWalkSpeed _player (/ (Variables|/Game/InteractionSystem/ThirdPersonBP/Blueprints/BP_InteractionTPC.BP_InteractionTPC_C|GetWalkSpeed _player) _multiplier))
      (Variables|/Game/InteractionSystem/ThirdPersonBP/Blueprints/BP_InteractionTPC.BP_InteractionTPC_C|SetRunSpeed _player (/ (Variables|/Game/InteractionSystem/ThirdPersonBP/Blueprints/BP_InteractionTPC.BP_InteractionTPC_C|GetRunSpeed _player) _multiplier))
      (Variables|/Script/Engine.CharacterMovementComponent|SetMaxWalkSpeed (Variables|/Script/Engine.Character|GetCharacterMovement _player) (/ (Variables|/Game/InteractionSystem/ThirdPersonBP/Blueprints/BP_InteractionTPC.BP_InteractionTPC_C|GetWalkSpeed _player) _multiplier)))))

(fn JumpReset
  (bind _player (Variables|Default|GetPlayer))
  (Utilities|IsValid _player
    (:Is%20Valid
      (Variables|/Script/Engine.CharacterMovementComponent|SetJumpZVelocity (Variables|/Script/Engine.Character|GetCharacterMovement _player) (Variables|/Game/InteractionSystem/ThirdPersonBP/Blueprints/BP_InteractionTPC.BP_InteractionTPC_C|GetDefaultJumpHeight _player)))))

(fn JumpCountReset
  (bind _player (Variables|Default|GetPlayer))
  (Utilities|IsValid _player
    (:Is%20Valid
      (Variables|/Script/Engine.Character|SetJumpMaxCount _player (- (Variables|/Script/Engine.Character|GetJumpMaxCount _player) (Math|Float|Truncate (Variables|Default|GetMultiplier)))))))

(fn DashReset
  (bind _player (Variables|Default|GetPlayer))
  (Utilities|IsValid _player
    (:Is%20Valid
      (Variables|/Game/InteractionSystem/ThirdPersonBP/Blueprints/BP_InteractionTPC.BP_InteractionTPC_C|SetDashAmount _player (/ (Variables|/Game/InteractionSystem/ThirdPersonBP/Blueprints/BP_InteractionTPC.BP_InteractionTPC_C|GetDashAmount _player) (Variables|Default|GetMultiplier))))))

(fn PickedUp
  (Variables|Default|SetCanPickup false)
  (Rendering|SetVisibility (Variables|Default|GetStaticMesh) false true))

(fn PickupReset
  (Variables|Default|SetCanPickup true)
  (Rendering|SetVisibility (Variables|Default|GetStaticMesh) true true))