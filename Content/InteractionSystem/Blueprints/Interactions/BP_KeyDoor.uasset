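; BP_KeyDoor is a locked door that opens when a player-controlled actor overlaps its box and KeyCollected is true, otherwise printing a prompt.
; A timeline swings DoorPivot in either direction with sounds, optionally reversing after a delay to close.
; The construction script applies the door material and key mesh.
; The key trigger's overlap event is empty; pickup logic that sets KeyCollected and destroys the key is disconnected.
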(event `self.Box.OnComponentBeginOverlap`
  (params (OverlappedComponent :type "PrimitiveComponent Object Reference") (OtherActor :type "Actor Object Reference") (OtherComp :type "PrimitiveComponent Object Reference") (OtherBodyIndex :type Integer) (bFromSweep :type Boolean) (SweepResult :type "HitResult Structure (by ref)"))
  (if (`Pawn.IsPlayerControlled` (`Actor.Instigator` OtherActor))
    (if (`self.KeyCollected`)
      (if (`self.DoorClosed`)
        (set `self.DoorClosed` false)
        (`GameplayStatics.SpawnSoundAtLocation` (`self.DoorOpenSound`) (`self.K2_GetActorLocation`) (struct) 1.0 1.0 0.0 (`self.Attenuation`) null)
        (bind (_direction _dooropen) (`Timeline|Timeline_0` :!label _label)
          (:`Update`
            (`SceneComponent.K2_SetRelativeRotation` (`self.DoorPivot`) (`KismetMathLibrary.MakeRotator` 0.0 0.0 (/ _dooropen (select `bool` (`self.OpenForward`) :`false` 1.0 :`true` -1.0))) false false))
          (:`Finished`
            (if (`self.CloseAfterOpen`)
              (`KismetSystemLibrary.Delay` (`self.DelayBeforeClose`))
              (set `self.DoorClosed` true)
              (`GameplayStatics.SpawnSoundAtLocation` (`self.DoorCloseSound`) (`self.K2_GetActorLocation`) (struct) 1.0 1.0 0.0 (`self.Attenuation`) null)
              (goto _label :!via `Reverse`)))))
      (else
        (`KismetSystemLibrary.PrintString` "You must first collect the key!" true true (struct :`R` 1.0 :`A` 1.0))))))

(event `self.KeyTrig.OnComponentBeginOverlap`
  (params (OverlappedComponent :type "PrimitiveComponent Object Reference") (OtherActor :type "Actor Object Reference") (OtherComp :type "PrimitiveComponent Object Reference") (OtherBodyIndex :type Integer) (bFromSweep :type Boolean) (SweepResult :type "HitResult Structure (by ref)")))

(fn `UserConstructionScript`
  (`PrimitiveComponent.SetMaterial` (`self.Door`) 0 (`self.Material`))
  (`StaticMeshComponent.SetStaticMesh` (`self.Key`) (`self.KeyMesh`)))