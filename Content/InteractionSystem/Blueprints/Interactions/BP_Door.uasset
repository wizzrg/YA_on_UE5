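; BP_Door is an interactable door that swings open on Interact and can close itself after a delay.
; The DoorOpen timeline drives the DoorPivot yaw, with OpenForward choosing the swing direction, and sounds play at the door.
; When the timeline finishes, a FlipFlop alternates between a DoOnce-guarded auto-close, which reverses the timeline if CloseAfterOpen is set, and resetting that DoOnce.
; The construction script applies the configurable material to the door mesh.
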(event `/Game/InteractionSystem/Blueprints/Master/BP_InteractInterface.Interact`
  (`GameplayStatics.SpawnSoundAtLocation` (`self.DoorOpenSound`) (`self.K2_GetActorLocation`) (struct) 1.0 1.0 0.0 (`self.Attenuation`) null)
  (bind (_direction _dooropen) (`Timeline|DoorOpen` :!label _label)
    (:`Update`
      (`SceneComponent.K2_SetRelativeRotation` (`self.DoorPivot`) (`KismetMathLibrary.MakeRotator` 0.0 0.0 (/ _dooropen (select `bool` (`self.OpenForward`) :`false` 1.0 :`true` -1.0 :!type "Float (single-precision)"))) false false))
    (:`Finished`
      (`/Engine/EditorBlueprintResources/StandardMacros.FlipFlop`
        (:`A`
          (`/Engine/EditorBlueprintResources/StandardMacros.DoOnce` false :!label _label_2
            (:`Completed`
              (if (`self.CloseAfterOpen`)
                (`KismetSystemLibrary.Delay` (`self.DelayBeforeClose`))
                (`GameplayStatics.SpawnSoundAtLocation` (`self.DoorCloseSound`) (`self.K2_GetActorLocation`) (struct) 1.0 1.0 0.0 (`self.Attenuation`) null)
                (goto _label :!via `Reverse`)))))
        (:`B`
          (goto _label_2 :!via `Reset`))))))

(fn `UserConstructionScript`
  (`PrimitiveComponent.SetMaterial` (`self.DoorMesh`) 0 (`self.Material`)))