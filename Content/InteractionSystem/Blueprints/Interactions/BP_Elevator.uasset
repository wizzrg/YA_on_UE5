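; Interactable elevator that moves its Elevator component to a configured relative location and rotation when Interact fires, playing an attenuated sound.
; A non-zero return delay sends it back to the transform cached at BeginPlay with a return sound, and the Loop option re-triggers Interact after a further delay.
; Separate editor events preview the move and reset it, while the construction script applies the configurable material.
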(event `self.ReceiveBeginPlay`
  ;[0.06477 1 0] Begin play
  (set `self.StartTransform` (`SceneComponent.GetRelativeTransform` (`self.Elevator`))))

(event `/Game/InteractionSystem/Blueprints/Master/BP_InteractInterface.Interact`
  (bind (_starttransform_location _starttransform_rotation) (`KismetMathLibrary.BreakTransform` (`self.StartTransform`)))
  (bind _returndelay (`self.ReturnDelay`))
  ;[1 1 1] Interact event
  (`GameplayStatics.SpawnSoundAtLocation` (`self.ElevatorActiveSound`) (`self.K2_GetActorLocation`) (struct) 1.0 1.0 0.0 (`self.Attenuation`) null)
  (`KismetSystemLibrary.MoveComponentTo` (`self.Elevator`) (`self.DistanceToMove`) (`self.Rotation`) false false (`self.TravelTime`))
  (if (not (== _returndelay 0.0))
    (`KismetSystemLibrary.Delay` _returndelay)
    (`GameplayStatics.SpawnSoundAtLocation` (`self.ElevatorReturnSound`) (`self.K2_GetActorLocation`) (struct) 1.0 1.0 0.0 (`self.Attenuation`) null)
    (`KismetSystemLibrary.MoveComponentTo` (`self.Elevator`) _starttransform_location _starttransform_rotation false false (`self.ReturnTravelTime`))
    (if (`self.Loop?`)
      (`KismetSystemLibrary.Delay` (`self.LoopDelay`))
      (`/Game/InteractionSystem/Blueprints/Master/BP_InteractInterface.Interact`))))

(event `PreviewMoveLoc`
  ;[1 1 1] Editor events
  (`KismetSystemLibrary.MoveComponentTo` (`self.Elevator`) (`self.DistanceToMove`) (`self.Rotation`) false false (`self.TravelTime`)))

(event `ResetElevatorLoc`
  (bind (_starttransform_location _starttransform_rotation) (`KismetMathLibrary.BreakTransform` (`self.StartTransform`)))
  ;[1 1 1] Editor events
  (`KismetSystemLibrary.MoveComponentTo` (`self.Elevator`) _starttransform_location _starttransform_rotation false false (`self.ReturnTravelTime`)))

(fn `UserConstructionScript`
  (`parent.UserConstructionScript`)
  (`PrimitiveComponent.SetMaterial` (`self.Elevator`) 0 (`self.Material`)))