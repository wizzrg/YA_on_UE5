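; BP_POI is an interaction actor for a point of interest that stays hidden until it is interacted with.
; BeginPlay hides the mesh and its text, and Interact reveals both and plays an attenuated activation sound at the actor's location.
; The construction script gives the mesh a dynamic instance of M_RenderThrough, tinted by the Colour variable.
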(event `self.ReceiveBeginPlay`
  (`SceneComponent.SetVisibility` (`self.StaticMesh`) false false)
  (`SceneComponent.SetVisibility` (`self.POIText`) false false))

(event `/Game/InteractionSystem/Blueprints/Master/BP_InteractInterface.Interact`
  (`SceneComponent.SetVisibility` (`self.StaticMesh`) true false)
  (`SceneComponent.SetVisibility` (`self.POIText`) true false)
  (`GameplayStatics.SpawnSoundAtLocation` (`self.ActivatedSound`) (`self.K2_GetActorLocation`) (struct) 1.0 1.0 0.0 (`self.Attenuation`) null))

(fn `UserConstructionScript`
  (locals (DynamicMatInst :type "MaterialInstanceDynamic Object Reference"))
  (`parent.UserConstructionScript`)
  (bind _returnvalue (`KismetMaterialLibrary.CreateDynamicMaterialInstance` "/Game/InteractionSystem/Materials/M_RenderThrough.M_RenderThrough"))
  (bind _output_get (set `local.DynamicMatInst` _returnvalue))
  (`PrimitiveComponent.SetMaterial` (`self.StaticMesh`) 0 _output_get)
  (`MaterialInstanceDynamic.SetVectorParameterValue` (`local.DynamicMatInst`) "Colour" (`self.Colour`)))