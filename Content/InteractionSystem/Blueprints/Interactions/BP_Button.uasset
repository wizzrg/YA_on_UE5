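; BP_Button is a pressure button that triggers its linked InteractActor list when a player-controlled actor overlaps its box.
; For each linked actor, it calls InteractMessage, turns the cylinder green, plays a pressed sound, and chains latent moves down and up before restoring red.
; A separate ConnectedActor event draws temporary debug lines from the button to each linked actor.
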(event `ConnectedActor`
  (bind _interactactor (`self.InteractActor`))
  ;[1 1 1] Debug line event
  (for _array_element _interactactor
    (if (== (`KismetArrayLibrary.Array_Length` _interactactor) 0)
      (`KismetSystemLibrary.PrintString` "Please select an interact actor first" true true (struct :`R` 1.0 :`B` 0.008376 :`A` 1.0) 3.0)
      (else
        (`KismetSystemLibrary.DrawDebugLine` (`SceneComponent.K2_GetComponentLocation` (`self.DefaultSceneRoot`)) (`SceneComponent.K2_GetComponentLocation` (`/Game/InteractionSystem/Blueprints/Master/BP_InteractMaster.DefaultSceneRoot` _array_element)) (struct :`R` 0.006271 :`G` 1.0 :`A` 1.0) 3.0 2.0)))))

(event `self.Box.OnComponentBeginOverlap`
  (params (OverlappedComponent :type "PrimitiveComponent Object Reference") (OtherActor :type "Actor Object Reference") (OtherComp :type "PrimitiveComponent Object Reference") (OtherBodyIndex :type Integer) (bFromSweep :type Boolean) (SweepResult :type "HitResult Structure (by ref)"))
  (bind _cylinder (`self.Cylinder`))
  ;[1 1 1] Overlap event
  (if (`Pawn.IsPlayerControlled` (`Actor.Instigator` OtherActor))
    (for _array_element (`self.InteractActor`)
      (message `/Game/InteractionSystem/Blueprints/Master/BP_InteractInterface.Interact` _array_element)
      (`PrimitiveComponent.SetMaterial` _cylinder 0 "/Game/InteractionSystem/Materials/SolidColours/MI_Green.MI_Green")
      (`GameplayStatics.SpawnSoundAtLocation` (`self.ButtonPressedSound`) (`self.K2_GetActorLocation`) (struct) 1.0 1.0 0.0 (`self.Attenuation`) null)
      (`KismetSystemLibrary.MoveComponentTo` _cylinder (0.0 0.0 -5.0) (struct) false false 0.5)
      (`KismetSystemLibrary.MoveComponentTo` (`self.Cylinder`) (0.0 0.0 5.0) (struct) false false 0.5)
      (`PrimitiveComponent.SetMaterial` (`self.Cylinder`) 0 "/Game/InteractionSystem/Materials/SolidColours/MI_Red.MI_Red"))))

(fn `UserConstructionScript`)