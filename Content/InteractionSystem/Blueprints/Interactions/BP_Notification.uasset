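; BP_Notification is an interactable actor that shows an on-screen text notification with a sound.
; It fires on Interact or when BP_InteractionTPC overlaps its Box, and the Box is destroyed at BeginPlay when ActivatedByButton is set.
; Both paths create a WBP_Notification widget with the configured text and colours, then play ActivatedSound at the actor's location with attenuation.
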(event `self.ReceiveBeginPlay`
  (if (`self.ActivatedByButton`)
    (`ActorComponent.K2_DestroyComponent` (`self.Box`))))

(event `/Game/InteractionSystem/Blueprints/Master/BP_InteractInterface.Interact`
  (bind _returnvalue (`|CreateWidget` "/Game/InteractionSystem/Widgets/WBP_Notification.WBP_Notification_C" null (`self.NotificationText`) (`self.TextColour`) (`self.BackgroundColour`) :!label _label))
  (`UserWidget.AddToViewport` _returnvalue 0)
  (`GameplayStatics.SpawnSoundAtLocation` (`self.ActivatedSound`) (`self.K2_GetActorLocation`) (struct) 1.0 1.0 0.0 (`self.Attenuation`) null))

(event `self.Box.OnComponentBeginOverlap`
  (params (OverlappedComponent :type "PrimitiveComponent Object Reference") (OtherActor :type "Actor Object Reference") (OtherComp :type "PrimitiveComponent Object Reference") (OtherBodyIndex :type Integer) (bFromSweep :type Boolean) (SweepResult :type "HitResult Structure (by ref)"))
  (cast `/Game/InteractionSystem/ThirdPersonBP/Blueprints/BP_InteractionTPC` OtherActor)
  (goto _label))

(fn `UserConstructionScript`)