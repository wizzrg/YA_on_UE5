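; BP_Sign is a configurable world sign built from a Cube panel and a TextRender label, with no runtime logic.
; The construction script applies the text, size and colour to the label and scales the cube to the set width and height, flattened to zero depth.
; It also gives the cube a dynamic instance of M_ColourMaster, driven by sign colour, glow colour and glow strength.
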(fn `UserConstructionScript`
  (locals (DynamMat :type "MaterialInstanceDynamic Object Reference"))
  (`TextRenderComponent.K2_SetText` (`self.TextRender`) (`self.Text`))
  (`SceneComponent.SetWorldScale3D` (`self.Cube`) (`KismetMathLibrary.MakeVector` (`self.Xsize`) 0.0 (`self.Zsize`)))
  (`TextRenderComponent.SetWorldSize` (`self.TextRender`) (`self.TextSize`))
  (`TextRenderComponent.SetTextRenderColor` (`self.TextRender`) (`self.TextColour`))
  (bind _returnvalue (`KismetMaterialLibrary.CreateDynamicMaterialInstance` "/Game/InteractionSystem/Materials/SolidColours/M_ColourMaster.M_ColourMaster"))
  (bind _output_get (set `local.DynamMat` _returnvalue))
  (`PrimitiveComponent.SetMaterial` (`self.Cube`) 0 _output_get)
  (`MaterialInstanceDynamic.SetVectorParameterValue` _output_get "Colour" (`self.SignColour`))
  (`MaterialInstanceDynamic.SetVectorParameterValue` _output_get "GlowColour" (`self.SignGlowColour`))
  (`MaterialInstanceDynamic.SetScalarParameterValue` _output_get "GlowStrength" (`self.SignGlowStrength`)))