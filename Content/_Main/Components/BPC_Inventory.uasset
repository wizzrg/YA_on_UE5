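; Player inventory component that stores minerals, potions and food in fixed slot arrays and tracks gold and artefact totals.
; Each tick a forward sphere trace toggles the item prompt widget, and the interact input adds the found item, destroys it and refreshes the inventory UI.
; Items stack up to DataTable limits before taking empty slots.
; Gold and artefacts are collected on capsule overlap, with amounts read from DataTables.
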(event `self.ReceiveTick`
  (params (DeltaSeconds :type "Float (single-precision)"))
  (bind _wbp_interactref (`self.WBP_InteractRef`))
  (bind (_item _founditem_) (`self.TraceItemToPickUp`))
  (set `/Game/_Main/UI_Widgets/WBP_ItemInfo.Item` _item (`/Game/_Main/UI_Widgets/WBP_Interact.WBP_ItemInfo` (`self.WBP_InteractRef`)))
  (if _founditem_
    (`UserWidget.AddToViewport` _wbp_interactref 0)
    (else
      (`Widget.RemoveFromParent` _wbp_interactref))))

(event `self.ReceiveBeginPlay`
  (bind (_minerals _potions _food) (break `/Game/_Main/Blueprints/Structures/S_AllItems` (`self.AllItems`)))
  (bind _asbp_player (cast `/Game/_Main/Player/BP_Player` (`GameplayStatics.GetPlayerCharacter` 0)))
  (set `self.PlayerRef` _asbp_player)
  (add `PrimitiveComponent.OnComponentBeginOverlap` (`Character.CapsuleComponent` (`self.PlayerRef`)) (`|CreateDelegate` :!event `PickUpGold`))
  (bind _returnvalue (`|CreateWidget` "/Game/_Main/UI_Widgets/WBP_Inventory_YA.WBP_Inventory_YA_C"))
  (set `self.InventoryYARef` _returnvalue)
  (add `PrimitiveComponent.OnComponentBeginOverlap` (`Character.CapsuleComponent` (`self.PlayerRef`)) (`|CreateDelegate` :!event `PickUpArtefact`))
  (bind _returnvalue_2 (`|CreateWidget` "/Game/_Main/UI_Widgets/WBP_Interact.WBP_Interact_C"))
  (set `self.WBP_InteractRef` _returnvalue_2)
  (`KismetArrayLibrary.Array_Resize` _minerals 12)
  (`KismetArrayLibrary.Array_Resize` _potions 12)
  (`KismetArrayLibrary.Array_Resize` _food 12)
  (`/Game/_Main/UI_Widgets/WBP_Inventory_YA.UpdateItemInInventoryUI` (`self.InventoryYARef`) (`self.AllItems`)))

(event `EnhancedInput|/Game/TopDown/Input/Actions/IA_Inventory`
  (params (ActionValue :type Boolean) (ElapsedSeconds :type "Float (double-precision)") (TriggeredSeconds :type "Float (double-precision)") (InputAction :type "InputAction Object Reference" :default "/Game/TopDown/Input/Actions/IA_Inventory.IA_Inventory"))
  (bind _returnvalue (`GameplayStatics.GetPlayerController` 0))
  (bind _inventoryyaref (`self.InventoryYARef`))
  (:`Triggered`
    (`UserWidget.AddToViewport` _inventoryyaref 0)
    (set `PlayerController.bShowMouseCursor` true _returnvalue)
    (`WidgetBlueprintLibrary.SetInputMode_UIOnlyEx` _returnvalue _inventoryyaref)))

(event `EnhancedInput|/Game/TopDown/Input/Actions/IA_Interact`
  (params (ActionValue :type Boolean) (ElapsedSeconds :type "Float (double-precision)") (TriggeredSeconds :type "Float (double-precision)") (InputAction :type "InputAction Object Reference" :default "/Game/TopDown/Input/Actions/IA_Interact.IA_Interact"))
  (:`Triggered`
    (bind (_item _founditem_ _itemactor) (`self.TraceItemToPickUp`))
    (if _founditem_
      (bind _success (`self.AddItemToInventory` _item))
      (if _success
        (`Actor.K2_DestroyActor` _itemactor)
        (`/Game/_Main/UI_Widgets/WBP_Inventory_YA.UpdateItemInInventoryUI` (`self.InventoryYARef`) (`self.AllItems`))))))

(fn `AddItemToInventory`
  (params (Item :type "/Game/_Main/Inventory/InventoryStructures/S_Slot Structure"))
  (returns (Success :type Boolean))
  (bind (_itemid _quantityamount _itemtype) (break `/Game/_Main/Inventory/InventoryStructures/S_Slot` (`local.Item`)))
  (bind (_itemid_2 _quantityamount_2) (break `/Game/_Main/Inventory/InventoryStructures/S_Slot` (`local.Item`)))
  (bind (_itemid_3 _quantityamount_3 _itemtype_2) (break `/Game/_Main/Inventory/InventoryStructures/S_Slot` (`local.Item`)))
  (bind (_itemid_4 _quantityamount_4) (break `/Game/_Main/Inventory/InventoryStructures/S_Slot` (`local.Item`)))
  (bind (_itemid_5 _quantityamount_5) (break `/Game/_Main/Inventory/InventoryStructures/S_Slot` (`local.Item`)))
  (bind (_itemid_6 _quantityamount_6 _itemtype_3) (break `/Game/_Main/Inventory/InventoryStructures/S_Slot` (`local.Item`)))
  (switch `/Game/_Main/Inventory/Enums/E_ItemTypes` (`.ItemType_8_5D91600A44B9B5D598ABD99473B587CF` (break `/Game/_Main/Inventory/InventoryStructures/S_Slot` Item))
    (:`NewEnumerator0`
      (`KismetSystemLibrary.PrintString` "Minerals")
      ;[1 1 1] Inventory Array Slot
      (for (_array_element _array_index) (`.Minerals_8_B183667D4023916E4E6D38B38CBEE650` (break `/Game/_Main/Blueprints/Structures/S_AllItems` (`self.AllItems`)))
        (bind (_itemid_7 _quantityamount_7) (break `/Game/_Main/Inventory/InventoryStructures/S_Slot` _array_element))
        (if (== (`.RowName` (break `DataTableRowHandle` _itemid_7)) (`.RowName` (break `DataTableRowHandle` (`.ItemID_2_06BDDC7D4036E6EBC56F39BB1983B212` (break `/Game/_Main/Inventory/InventoryStructures/S_Slot` (`local.Item`))))))
          (bind _returnvalue (`|GetDataTableRow` "/Game/_Main/Inventory/DataTables/DT_ItemMaster.DT_ItemMaster" (`.RowName` (break `DataTableRowHandle` _itemid_2)))
            (:`then`
              (bind _returnvalue_2 (+ _quantityamount_2 _quantityamount_7))
              (if (>= (`.StackSize_13_C1476B4F4B3B94A93A78EDA7E4F52F58` (break `/Game/_Main/Blueprints/Structures/S_ItemMaster` _returnvalue)) _returnvalue_2)
                (`KismetArrayLibrary.Array_Set` (`.Minerals_8_B183667D4023916E4E6D38B38CBEE650` (break `/Game/_Main/Blueprints/Structures/S_AllItems` (`self.AllItems`))) _array_index (make `/Game/_Main/Inventory/InventoryStructures/S_Slot` _itemid _returnvalue_2 _itemtype))
                (return true))))))
      (for (_array_element_2 _array_index_2) (`.Minerals_8_B183667D4023916E4E6D38B38CBEE650` (break `/Game/_Main/Blueprints/Structures/S_AllItems` (`self.AllItems`)))
        (if (== (`.QuantityAmount_5_F7B1BF8B4702BEEE0C73B1990E8CD63A` (break `/Game/_Main/Inventory/InventoryStructures/S_Slot` _array_element_2)) 0)
          (`KismetArrayLibrary.Array_Set` (`.Minerals_8_B183667D4023916E4E6D38B38CBEE650` (break `/Game/_Main/Blueprints/Structures/S_AllItems` (`self.AllItems`))) _array_index_2 (`local.Item`))
          (return true)))
      (return false))
    (:`NewEnumerator1`
      (for (_array_element_3 _array_index_3) (`.Potions_9_F1118601420A30DC4E5EEFB2DBA44B9D` (break `/Game/_Main/Blueprints/Structures/S_AllItems` (`self.AllItems`)))
        (bind (_itemid_8 _quantityamount_8) (break `/Game/_Main/Inventory/InventoryStructures/S_Slot` _array_element_3))
        (if (== (`.RowName` (break `DataTableRowHandle` _itemid_8)) (`.RowName` (break `DataTableRowHandle` (`.ItemID_2_06BDDC7D4036E6EBC56F39BB1983B212` (break `/Game/_Main/Inventory/InventoryStructures/S_Slot` (`local.Item`))))))
          (bind _returnvalue_3 (`|GetDataTableRow` "/Game/_Main/Inventory/DataTables/DT_ItemMaster.DT_ItemMaster" (`.RowName` (break `DataTableRowHandle` _itemid_4)))
            (:`then`
              (bind _returnvalue_4 (+ _quantityamount_4 _quantityamount_8))
              (if (>= (`.StackSize_13_C1476B4F4B3B94A93A78EDA7E4F52F58` (break `/Game/_Main/Blueprints/Structures/S_ItemMaster` _returnvalue_3)) _returnvalue_4)
                (`KismetArrayLibrary.Array_Set` (`.Potions_9_F1118601420A30DC4E5EEFB2DBA44B9D` (break `/Game/_Main/Blueprints/Structures/S_AllItems` (`self.AllItems`))) _array_index_3 (make `/Game/_Main/Inventory/InventoryStructures/S_Slot` _itemid_6 _returnvalue_4 _itemtype_3))
                (return true))))))
      (for (_array_element_4 _array_index_4) (`.Potions_9_F1118601420A30DC4E5EEFB2DBA44B9D` (break `/Game/_Main/Blueprints/Structures/S_AllItems` (`self.AllItems`)))
        (if (== (`.QuantityAmount_5_F7B1BF8B4702BEEE0C73B1990E8CD63A` (break `/Game/_Main/Inventory/InventoryStructures/S_Slot` _array_element_4)) 0)
          (`KismetArrayLibrary.Array_Set` (`.Potions_9_F1118601420A30DC4E5EEFB2DBA44B9D` (break `/Game/_Main/Blueprints/Structures/S_AllItems` (`self.AllItems`))) _array_index_4 (`local.Item`))
          (return true)))
      (return false))
    (:`NewEnumerator2`
      (for (_array_element_5 _array_index_5) (`.Food_10_C97249AB4CAD1ACBA1F7BEAFF0BB228C` (break `/Game/_Main/Blueprints/Structures/S_AllItems` (`self.AllItems`)))
        (bind (_itemid_9 _quantityamount_9) (break `/Game/_Main/Inventory/InventoryStructures/S_Slot` _array_element_5))
        (if (== (`.RowName` (break `DataTableRowHandle` _itemid_9)) (`.RowName` (break `DataTableRowHandle` (`.ItemID_2_06BDDC7D4036E6EBC56F39BB1983B212` (break `/Game/_Main/Inventory/InventoryStructures/S_Slot` (`local.Item`))))))
          (bind _returnvalue_5 (`|GetDataTableRow` "/Game/_Main/Inventory/DataTables/DT_ItemMaster.DT_ItemMaster" (`.RowName` (break `DataTableRowHandle` _itemid_5)))
            (:`then`
              (bind _returnvalue_6 (+ _quantityamount_5 _quantityamount_9))
              (if (>= (`.StackSize_13_C1476B4F4B3B94A93A78EDA7E4F52F58` (break `/Game/_Main/Blueprints/Structures/S_ItemMaster` _returnvalue_5)) _returnvalue_6)
                (`KismetArrayLibrary.Array_Set` (`.Food_10_C97249AB4CAD1ACBA1F7BEAFF0BB228C` (break `/Game/_Main/Blueprints/Structures/S_AllItems` (`self.AllItems`))) _array_index_5 (make `/Game/_Main/Inventory/InventoryStructures/S_Slot` _itemid_3 _returnvalue_6 _itemtype_2))
                (return true))))))
      (for (_array_element_6 _array_index_6) (`.Food_10_C97249AB4CAD1ACBA1F7BEAFF0BB228C` (break `/Game/_Main/Blueprints/Structures/S_AllItems` (`self.AllItems`)))
        (if (== (`.QuantityAmount_5_F7B1BF8B4702BEEE0C73B1990E8CD63A` (break `/Game/_Main/Inventory/InventoryStructures/S_Slot` _array_element_6)) 0)
          (`KismetArrayLibrary.Array_Set` (`.Food_10_C97249AB4CAD1ACBA1F7BEAFF0BB228C` (break `/Game/_Main/Blueprints/Structures/S_AllItems` (`self.AllItems`))) _array_index_6 (`local.Item`))
          (return true)))
      (return false))))

(fn `PickUpArtefact`
  (params (OverlappedComponent :type "PrimitiveComponent Object Reference") (OtherActor :type "Actor Object Reference") (OtherComp :type "PrimitiveComponent Object Reference") (OtherBodyIndex :type Integer) (bFromSweep :type Boolean) (SweepResult :type "HitResult Structure (by ref)"))
  (bind _asbp_artefact_master (cast `/Game/_Main/Inventory/Artefacts/BP_Artefact_Master` OtherActor))
  (bind (_artefactdt_datatable _artefactdt_rowname) (break `DataTableRowHandle` (`/Game/_Main/Inventory/Artefacts/BP_Artefact_Master.ArtefactDT` _asbp_artefact_master)))
  (bind _returnvalue (`|GetDataTableRow` "/Game/_Main/Inventory/DataTables/DT_Artefact.DT_Artefact" _artefactdt_rowname)
    (:`then`
      (bind _output_get (set `self.ArtefactAmountComponent` (+ (`.Amount_7_5BF8295A4E62C94C988F198E46C365D6` (break `/Game/_Main/Blueprints/Structures/S_Artefacts` _returnvalue)) (`self.ArtefactAmountComponent`))))
      (`KismetSystemLibrary.PrintString` (`KismetStringLibrary.Conv_IntToString` _output_get))
      (set `/Game/_Main/UI_Widgets/WBP_Inventory_YA.ArtefactAmountWidget` (`self.ArtefactAmountComponent`) (`self.InventoryYARef`))
      (`Actor.K2_DestroyActor` _asbp_artefact_master)
      (return))))

(fn `PickUpGold`
  (params (OverlappedComponent :type "PrimitiveComponent Object Reference") (OtherActor :type "Actor Object Reference") (OtherComp :type "PrimitiveComponent Object Reference") (OtherBodyIndex :type Integer) (bFromSweep :type Boolean) (SweepResult :type "HitResult Structure (by ref)"))
  (bind _asbp_gold_master (cast `/Game/_Main/Inventory/Gold/BP_Gold_Master` OtherActor))
  (bind (_gold_datatable _gold_rowname) (break `DataTableRowHandle` (`/Game/_Main/Inventory/Gold/BP_Gold_Master.Gold` _asbp_gold_master)))
  (bind _returnvalue (`|GetDataTableRow` "/Game/_Main/Inventory/DataTables/DT_Gold.DT_Gold" _gold_rowname)
    (:`then`
      (bind _output_get (set `self.GoldAmountComponent` (+ (`.Amount_7_ADD076E24F078873E83B2A9E5001BBBF` (break `/Game/_Main/Blueprints/Structures/S_Gold` _returnvalue)) (`self.GoldAmountComponent`))))
      (`KismetSystemLibrary.PrintString` (`KismetStringLibrary.Conv_IntToString` _output_get))
      (set `/Game/_Main/UI_Widgets/WBP_Inventory_YA.GoldAmountWidget` (`self.GoldAmountComponent`) (`self.InventoryYARef`))
      (`Actor.K2_DestroyActor` _asbp_gold_master)
      (return))))

(fn `TraceItemToPickUp`
  (returns (Item :type "/Game/_Main/Inventory/InventoryStructures/S_Slot Structure") (`FoundItem?` :type Boolean) (ItemActor :type "Actor Object Reference"))
  (bind _returnvalue (`GameplayStatics.GetPlayerCharacter` 0))
  (bind _returnvalue_2 (- (`Actor.K2_GetActorLocation` _returnvalue) (0.0 0.0 0.0)))
  (bind _outhit (`KismetSystemLibrary.SphereTraceSingle` :`Start` _returnvalue_2 :`End` (+ _returnvalue_2 (* (`Actor.GetActorForwardVector` _returnvalue) 225.0)) :`Radius` 90.0 :`TraceChannel` "TraceTypeQuery1" :`DrawDebugType` "ForOneFrame"))
  (bind (_bblockinghit _binitialoverlap _time _distance _location _impactpoint _normal _impactnormal _physmat _hitactor) (`GameplayStatics.BreakHitResult` _outhit))
  (bind _asbp_item_master (cast `/Game/_Main/Inventory/Items/BP_ItemMaster` _hitactor)
    (:`then`
      (bind _output_get (set `self.ItemMasterRef` _asbp_item_master))
      (`/Engine/EditorBlueprintResources/StandardMacros.IsValid` _output_get
        (:`Is Valid`
          (return (`/Game/_Main/Inventory/Items/BP_ItemMaster.Item` _asbp_item_master) true _hitactor))))
    (:`CastFailed`
      (return (struct) false null))))