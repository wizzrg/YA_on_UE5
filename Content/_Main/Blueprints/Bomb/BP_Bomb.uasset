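; BP_Bomb is a timed bomb actor that deals radial explosion damage two seconds after it begins play.
; The Sphere component's radius sets the full-damage blast area and is drawn as a debug sphere every tick.
; The explosion particle, sound and actor destruction run only if the radial damage call reports a hit.
; A separate ApplyDamage call precedes the radial one with no damaged actor specified.
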(event `self.ReceiveTick`
  (params (DeltaSeconds :type "Float (single-precision)"))
  (bind _sphere (`self.Sphere`))
  (`KismetSystemLibrary.DrawDebugSphere` (`SceneComponent.K2_GetComponentLocation` _sphere) (`SphereComponent.SphereRadius` _sphere)))

(event `self.ReceiveBeginPlay`
  (bind _sm_stone01 (`self.SM_Stone01`))
  (bind _returnvalue (`SceneComponent.K2_GetComponentLocation` _sm_stone01))
  (`/Engine/EditorBlueprintResources/StandardMacros.IsValid` (`self.Sphere`)
    (:`Is Valid`
      (`KismetSystemLibrary.Delay` 2.0)
      (`GameplayStatics.ApplyDamage` null 2.0 null null "/Game/_Main/Blueprints/Bomb/DT_BombExplosion.DT_BombExplosion_C")
      (bind _returnvalue_2 (`GameplayStatics.ApplyRadialDamage` :`BaseDamage` 2.0 :`Origin` (`self.K2_GetActorLocation`) :`DamageRadius` (`SphereComponent.SphereRadius` (`self.Sphere`)) :`DamageTypeClass` "/Game/_Main/Blueprints/Bomb/DT_BombExplosion.DT_BombExplosion_C" :`DamageCauser` null :`InstigatedByController` null :`bDoFullDamage` true))
      (if _returnvalue_2
        (`GameplayStatics.SpawnEmitterAtLocation` "/Game/StarterContent/Particles/P_Explosion.P_Explosion" _returnvalue (`SceneComponent.K2_GetComponentRotation` _sm_stone01))
        (`GameplayStatics.PlaySoundAtLocation` "/Game/StarterContent/Audio/Explosion_Cue.Explosion_Cue" _returnvalue (struct) 1.0 1.0 0.0 null null null null)
        (`ActorComponent.Deactivate` (`self.Sphere`))
        (`self.K2_DestroyActor`)))))

(fn `UserConstructionScript`)