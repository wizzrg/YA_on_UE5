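; Master pickup item that grants the player temporary lives on overlapping its sphere, which is drawn as a debug sphere every tick.
; Pickup requires no active temp lives and total lives below the base maximum.
; It saves base lives, adds temp lives, sets the player's timer and destroys itself.
; Active temp lives only trigger a message; older permanent-life and timer-array logic remains disconnected.
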(event `self.ReceiveBeginPlay`)

(event `self.ReceiveTick`
  (params (DeltaSeconds :type "Float (single-precision)"))
  (bind _sphere (`self.Sphere`))
  (`KismetSystemLibrary.DrawDebugSphere` (`SceneComponent.K2_GetComponentLocation` _sphere) (`SphereComponent.SphereRadius` _sphere) 12 (struct :`R` 1.0 :`G` 1.0 :`B` 1.0 :`A` 1.0) 0.0 1.0))

(event `self.Sphere.OnComponentBeginOverlap`
  (params (OverlappedComponent :type "PrimitiveComponent Object Reference") (OtherActor :type "Actor Object Reference") (OtherComp :type "PrimitiveComponent Object Reference") (OtherBodyIndex :type Integer) (bFromSweep :type Boolean) (SweepResult :type "HitResult Structure (by ref)"))
  (bind _playerref (`self.PlayerRef`))
  (bind _playerref_2 (`self.PlayerRef`))
  (bind _asbp_player (cast `/Game/_Main/Player/BP_Player` OtherActor))
  (bind _output_get (set `self.PlayerRef` _asbp_player))
  (`/Engine/EditorBlueprintResources/StandardMacros.IsValid` _output_get
    (:`Is Valid`
      (if (< (`/Game/_Main/Player/BP_Player.TempLives` _output_get) 1)
        (if (< (+ (`/Game/_Main/Player/BP_Player.BasePlayerLives` _playerref_2) (`/Game/_Main/Player/BP_Player.TempLives` _playerref_2)) (`/Game/_Main/Player/BP_Player.BaseMaxPlayerLives` _playerref_2))
          (if (== (`/Game/_Main/Player/BP_Player.TempLives` (`self.PlayerRef`)) 0)
            (set `/Game/_Main/Player/BP_Player.BaseLivesBeforeTemp` (`/Game/_Main/Player/BP_Player.BasePlayerLives` _playerref) _playerref)
            (set `/Game/_Main/Player/BP_Player.TempLives` (+ (`/Game/_Main/Player/BP_Player.TempLives` _playerref) (`self.TempLivesToAdd`)) _playerref)
            (set `/Game/_Main/Player/BP_Player.TempLiveTiimer` (`self.TempLivesDuration`) (`self.PlayerRef`))
            (`self.K2_DestroyActor`)))
        (else
          (`KismetSystemLibrary.PrintString` "You have full Temp Lives" true true (struct :`G` 1.0 :`B` 0.561116 :`A` 1.0)))))))

(fn `UserConstructionScript`)