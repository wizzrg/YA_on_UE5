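; BP_TestDamageCube is a test damage volume that hurts actors tagged Player or Enemy when they begin overlapping its Box component.
; Each qualifying overlap applies BaseDamage through the standard ApplyDamage call and prints an on-screen hit message.
; Tick draws a debug box at the Box's location and extent.
; Disconnected nodes that cast to BP_Player and subtract directly from its temporary or base lives never execute.
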(event `self.ReceiveTick`
  (params (DeltaSeconds :type "Float (single-precision)"))
  (bind _box (`self.Box`))
  (`KismetSystemLibrary.DrawDebugBox` (`SceneComponent.K2_GetComponentLocation` _box) (`BoxComponent.BoxExtent` _box)))

(event `self.Box.OnComponentBeginOverlap`
  (params (OverlappedComponent :type "PrimitiveComponent Object Reference") (OtherActor :type "Actor Object Reference") (OtherComp :type "PrimitiveComponent Object Reference") (OtherBodyIndex :type Integer) (bFromSweep :type Boolean) (SweepResult :type "HitResult Structure (by ref)"))
  (if (`KismetSystemLibrary.IsValid` OtherActor)
    (if (or (`self.ActorHasTag` OtherActor "Player") (`self.ActorHasTag` OtherActor "Enemy"))
      (`GameplayStatics.ApplyDamage` OtherActor (`KismetMathLibrary.Conv_IntToDouble` (`self.Base Damage`)))
      (`KismetSystemLibrary.PrintString` "You hitted by a Cube" true true (struct :`R` 0.108294 :`G` 1.0 :`B` 0.218351 :`A` 1.0)))))

(fn `UserConstructionScript`)