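; BP_Player is the player character, sliding in one of four directions until a hit or line trace frees it to turn.
; Tick drives the slide, temporary-life expiry and bomb cooldown shown on the HUD.
; Damage reduces temporary or base lives; death triggers ragdoll, game over and gold/artefact reset, and destruction calls the GameMode respawn.
; It also handles torch toggling, camera zoom and harvesting into the inventory component.
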(event Custom|TakeAnyDamage
  (params (DamagedActor :type Actor%20Object%20Reference) (Damage :type Float%20%28single-precision%29) (DamageType :type Damage%20Type%20Object%20Reference) (InstigatedBy :type Controller%20Object%20Reference) (DamageCauser :type Actor%20Object%20Reference))
  (bind _output_get (Variables|Default|SetDamageTakenValue Damage))
  (CallFunction|FPlayerTakeDamage _output_get)
  (Animation|Montage|PlayMontage (Variables|Character|GetMesh) "/Game/_Main/Player/YA_Character/Adam_Char/Animations/AM_HitReaction.AM_HitReaction"))

(event Custom|PlayerIsDead
  ;[1 1 1] Player is Dead
  (Variables|Default|SetisPlayerDead? true)
  (bind _returnvalue (UserInterface|CreateWidget "/Game/_Main/UI_Widgets/WBP_GameOver.WBP_GameOver_C"))
  (UserInterface|Viewport|AddtoViewport _returnvalue 0)
  (bind _returnvalue_2 (Actor|GetActorOfClass "/Script/Engine.CameraActor"))
  (Game|Player|SetViewTargetwithBlend (Game|GetPlayerController 0) _returnvalue_2 4.0 "VTBlend_Linear" 0.0 false)
  (bind _asbp_ya_game_instance (Utilities|Casting|CastToBP_YA_GameInstance (Game|GetGameInstance)))
  (Variables|/Game/_Main/Blueprints/BP_YA_GameInstance.BP_YA_GameInstance_C|SetGoldCount _asbp_ya_game_instance 0)
  (Variables|/Game/_Main/Blueprints/BP_YA_GameInstance.BP_YA_GameInstance_C|SetArtefactCount _asbp_ya_game_instance 0))

(event Custom|DestroyPlayer
  (params (Duration :type Float%20%28double-precision%29) (Target :type Actor%20Object%20Reference))
  (Variables|Default|SetisPlayerDead? true)
  (Utilities|DestroyPlayerMacros Duration Target))

(event Custom|EquipedItemMesh
  (params (Item :type S%20Craft%20Item%20Master%20Structure))
  (bind _equipped_item (Variables|Default|GetEquipped%20Item))
  ;[1 1 1] Equiped Item Mesh
  (if (not (Variables|Default|GetisPlayerDead?))
    (bind _returnvalue (Components|StaticMesh|SetStaticMesh _equipped_item (.StaticMesh (Utilities|Struct|BreakS_CraftItemMaster Item))))
    (if _returnvalue
      (if (not (Variables|Default|GetisPlayerDead?))
        (Collision|SetCollisionEnabled _equipped_item "NoCollision")))))

(event Input|EnhancedActionEvents|EnhancedInputActionIA_MoveUp
  (params (ActionValue :type Boolean) (ElapsedSeconds :type Float%20%28double-precision%29) (TriggeredSeconds :type Float%20%28double-precision%29) (InputAction :type Input%20Action%20Object%20Reference :default "/Game/TopDown/Input/Actions/IA_MoveUp.IA_MoveUp"))
  ;[1 1 1] Character Movement
  (:Triggered
    (if (Variables|PlayerMovement|GetCanChangeDirection)
      (Variables|PlayerMovement|SetIsMoving true)
      (Variables|PlayerMovement|SetMoveDirection "1.000000,0.000000,0.000000")
      (Pawn|Input|AddMovementInput (Variables|PlayerMovement|GetMoveDirection) 1.0 false)
      (Variables|PlayerMovement|SetCanChangeDirection false)))
  (:Canceled
    (Variables|PlayerMovement|SetIsMoving false :!label _label))
  (:Completed
    (goto _label)))

(event Input|EnhancedActionEvents|EnhancedInputActionIA_MoveDown
  (params (ActionValue :type Boolean) (ElapsedSeconds :type Float%20%28double-precision%29) (TriggeredSeconds :type Float%20%28double-precision%29) (InputAction :type Input%20Action%20Object%20Reference :default "/Game/TopDown/Input/Actions/IA_MoveDown.IA_MoveDown"))
  ;[1 1 1] Character Movement
  (:Triggered
    (if (Variables|PlayerMovement|GetCanChangeDirection)
      (Variables|PlayerMovement|SetIsMoving true)
      (Variables|PlayerMovement|SetMoveDirection "-1.000000,0.000000,0.000000")
      (Pawn|Input|AddMovementInput (Variables|PlayerMovement|GetMoveDirection) 1.0 false)
      (Variables|PlayerMovement|SetCanChangeDirection false)))
  (:Canceled
    (Variables|PlayerMovement|SetIsMoving false :!label _label))
  (:Completed
    (goto _label)))

(event Input|EnhancedActionEvents|EnhancedInputActionIA_MoveRight
  (params (ActionValue :type Boolean) (ElapsedSeconds :type Float%20%28double-precision%29) (TriggeredSeconds :type Float%20%28double-precision%29) (InputAction :type Input%20Action%20Object%20Reference :default "/Game/TopDown/Input/Actions/IA_MoveRight.IA_MoveRight"))
  ;[1 1 1] Character Movement
  (:Triggered
    (if (Variables|PlayerMovement|GetCanChangeDirection)
      (Variables|PlayerMovement|SetIsMoving true)
      (Variables|PlayerMovement|SetMoveDirection "0.000000,1.000000,0.000000")
      (Pawn|Input|AddMovementInput (Variables|PlayerMovement|GetMoveDirection) 1.0 false)
      (Variables|PlayerMovement|SetCanChangeDirection false)))
  (:Canceled
    (Variables|PlayerMovement|SetIsMoving false :!label _label))
  (:Completed
    (goto _label)))

(event Input|EnhancedActionEvents|EnhancedInputActionIA_MoveLeft
  (params (ActionValue :type Boolean) (ElapsedSeconds :type Float%20%28double-precision%29) (TriggeredSeconds :type Float%20%28double-precision%29) (InputAction :type Input%20Action%20Object%20Reference :default "/Game/TopDown/Input/Actions/IA_MoveLeft.IA_MoveLeft"))
  ;[1 1 1] Character Movement
  (:Triggered
    (if (Variables|PlayerMovement|GetCanChangeDirection)
      (Variables|PlayerMovement|SetIsMoving true)
      (Variables|PlayerMovement|SetMoveDirection "0.000000,-1.000000,0.000000")
      (Pawn|Input|AddMovementInput (Variables|PlayerMovement|GetMoveDirection) 1.0 false)
      (Variables|PlayerMovement|SetCanChangeDirection false)))
  (:Canceled
    (Variables|PlayerMovement|SetIsMoving false :!label _label))
  (:Completed
    (goto _label)))

(event Input|EnhancedActionEvents|EnhancedInputActionIA_Jump
  (params (ActionValue :type Boolean) (ElapsedSeconds :type Float%20%28double-precision%29) (TriggeredSeconds :type Float%20%28double-precision%29) (InputAction :type Input%20Action%20Object%20Reference :default "/Game/TopDown/Input/Actions/IA_Jump.IA_Jump"))
  ;[1 1 1] Character Movement
)

(event Input|EnhancedActionEvents|EnhancedInputActionIA_CameraZoom
  (params (ActionValue :type Float%20%28double-precision%29) (ElapsedSeconds :type Float%20%28double-precision%29) (TriggeredSeconds :type Float%20%28double-precision%29) (InputAction :type Input%20Action%20Object%20Reference :default "/Game/TopDown/Input/Actions/IA_CameraZoom.IA_CameraZoom"))
  ;[1 1 1] Character Movement
  (CallFunction|CameraZoom))

(event Input|EnhancedActionEvents|EnhancedInputActionIA_Interact
  (params (ActionValue :type Boolean) (ElapsedSeconds :type Float%20%28double-precision%29) (TriggeredSeconds :type Float%20%28double-precision%29) (InputAction :type Input%20Action%20Object%20Reference :default "/Game/TopDown/Input/Actions/IA_Interact.IA_Interact")))

(event Input|EnhancedActionEvents|EnhancedInputActionIA_Abilitie1
  (params (ActionValue :type Boolean) (ElapsedSeconds :type Float%20%28double-precision%29) (TriggeredSeconds :type Float%20%28double-precision%29) (InputAction :type Input%20Action%20Object%20Reference :default "/Game/TopDown/Input/Actions/IA_Abilitie1.IA_Abilitie1"))
  ;[1 1 1] Spawning Bomb Abbilitie
  (if (not (Variables|Default|GetisAbilitieTimerActive?))
    (if (Variables|Default|GetCanSpawnBomb)
      (CallFunction|FSpawnBombAbilitie)
      (Widget|SetVisibility (Variables|/Game/_Main/UI_Widgets/WBP_BombAbilitie.WBP_BombAbilitie_C|GetAbilitieTimerText (Variables|/Game/_Main/UI_Widgets/WBP_MainHUD.WBP_MainHUD_C|GetWBP_BombAbilitie (Variables|Default|GetMainHUDRef))) "Visible")
      (Variables|Default|SetCanSpawnBomb false)
      (Variables|Default|SetisAbilitieTimerActive? true)
      (Variables|Default|SetAbilitieCooldownTimer (Variables|Default|GetAbilitieCooldownTimer)))))

(event Input|EnhancedActionEvents|EnhancedInputActionIA_Torch
  (params (ActionValue :type Boolean) (ElapsedSeconds :type Float%20%28double-precision%29) (TriggeredSeconds :type Float%20%28double-precision%29) (InputAction :type Input%20Action%20Object%20Reference :default "/Game/TopDown/Input/Actions/IA_Torch.IA_Torch"))
  ;[1 1 1] Equip Torch
  (Utilities|FlowControl|FlipFlop
    (:A
      (bind _returnvalue (Game|SpawnActorfromClass "/Game/_Main/Blueprints/BP_Torch.BP_Torch_C" (Transformation|GetSocketTransform (Variables|Character|GetMesh) "TorchSocket" "RTS_World") "AlwaysSpawn" "MultiplyWithRoot" 0 0))
      (Transformation|AttachComponentToComponent _returnvalue (Variables|Character|GetMesh) "TorchSocket" "SnapToTarget" "SnapToTarget" "SnapToTarget" true))
    (:B
      (Transformation|DetachFromActor _returnvalue "KeepRelative" "KeepRelative" "KeepRelative")
      (Actor|DestroyActor _returnvalue))))

(event EventTick
  (params (DeltaSeconds :type Float%20%28single-precision%29))
  (CallFunction|FStopMovementLineTrace)
  (CallFunction|FRemoveTempLivesTimer DeltaSeconds)
  (CallFunction|FAbilitieOneTimer DeltaSeconds))

(event EventBeginPlay
  (Utilities|FlowControl|Sequence
    (:then_0
      (Variables|/Script/Engine.SpringArmComponent|SetTargetArmLength (Variables|Default|GetSpringArm) 6e+02))
    (:then_1
      (bind _returnvalue (UserInterface|CreateWidget "/Game/_Main/UI_Widgets/WBP_MainHUD.WBP_MainHUD_C" (Game|GetPlayerController 0)))
      (bind _output_get (Variables|Default|SetMainHUDRef _returnvalue))
      (UserInterface|Viewport|AddtoViewport _output_get 0))
    (:then_2
      (CallFunction|FSetPLayerHealth)
      (Variables|Default|SetAC_InventoryAndCrafting (Variables|Default|GetAC_InventoryAndCrafting))
      (Variables|Default|SetAbilitieCooldownTimer (Variables|Default|GetAbilitieCooldownTimer)))
    (:then_3
      (EventDispatchers|AssignOnTakeAnyDamage (delegate Custom|TakeAnyDamage)))))

(event Collision|EventHit
  (params (MyComp :type Primitive%20Component%20Object%20Reference) (Other :type Actor%20Object%20Reference) (OtherComp :type Primitive%20Component%20Object%20Reference) (bSelfMoved :type Boolean) (HitLocation :type Vector :default "0, 0, 0") (HitNormal :type Vector :default "0, 0, 0") (NormalImpulse :type Vector :default "0, 0, 0") (Hit :type Hit%20Result%20Structure%20%28by%20ref%29))
  (Variables|PlayerMovement|SetIsMoving false)
  (Variables|PlayerMovement|SetCanChangeDirection true))

(event EventHarvestItem
  (params (Item :type S%20Craft%20Item%20Master%20Structure))
  ;[1 1 1] Harvest Items
  (Default|AddItem (Variables|Default|GetAC_InventoryAndCrafting) Item))

(event EventDestroyed
  (bind _asbp_ya_game_mode (Utilities|Casting|CastToBP_YA_GameMode (Game|GetGameMode)))
  (Default|RespawnPlayer _asbp_ya_game_mode self))

(event EventInteract)

(event Input|KeyboardEvents|DebugKeyM
  (params (Key :type Key%20Structure :default "None") (ActionValue :type Input%20Action%20Value%20Structure))
  (:Pressed
    (Development|PrintText (Utilities|Text|FormatText "Current Player Lives: {0}" (Variables|Default|GetBasePlayerLives)))
    (Development|PrintText (Utilities|Text|FormatText "Current Temp Player Lives: {0}" (Variables|Default|GetTempLives)) true true "(R=0.091597,G=0.940270,B=1.000000,A=1.000000)")))

(fn ConstructionScript)

(fn CameraZoom
  (bind _springarm (Variables|Default|GetSpringArm))
  (Variables|/Script/Engine.SpringArmComponent|SetTargetArmLength _springarm (Math|Interpolation|FInterpTo (Variables|/Script/Engine.SpringArmComponent|GetTargetArmLength _springarm) (Math|Float|Clamp(Float) (+ (Variables|/Script/Engine.SpringArmComponent|GetTargetArmLength _springarm) (* (Input|AxisValues|GetZoomInOut) (Variables|CameraZoom|GetZoomSpeed))) (Variables|CameraZoom|GetMinZoom) (Variables|CameraZoom|GetMaxZoom)) (Utilities|Time|GetWorldDeltaSeconds) 5.0))
  (return))

(fn FSetPLayerHealth
  (Variables|Default|SetBasePlayerLives (Variables|Default|GetBasePlayerLives))
  (Variables|Default|SetBaseMaxPlayerLives (Variables|Default|GetBaseMaxPlayerLives))
  (Variables|Default|SetTempLives (Variables|Default|GetTempLives))
  (Variables|Default|SetBaseLivesBeforeTemp (Variables|Default|GetBaseLivesBeforeTemp))
  (Variables|Default|SetTempLiveTiimer (Variables|Default|GetTempLiveTiimer))
  (bind _returnvalue (Utilities|Time|SetTimerbyFunctionName 0 "PlayersDeath" 0.1))
  (Variables|Default|SetTimer _returnvalue)
  (return))

(fn FPlayersDeath
  (bind _mesh (Variables|Character|GetMesh))
  (if (<= (Variables|Default|GetBasePlayerLives) 0)
    (Physics|SetSimulatePhysics _mesh true)
    (Collision|SetCollisionProfileName _mesh "Ragdoll" true :!class /Script/Engine.PrimitiveComponent)
    (Collision|SetCollisionEnabled (Variables|Collision|GetCapsuleComponent) "NoCollision")
    (Utilities|Time|PauseTimerbyHandle (Variables|Default|GetTimer))
    (CallFunction|DestroyPlayer (Variables|Default|GetTimeDelay) self)
    (return)))

(fn FStopMovementLineTrace
  (bind _returnvalue (Transformation|GetActorLocation))
  (bind _stopdistance (Variables|PlayerMovement|GetStopDistance))
  (if (>= (Variables|/Script/Engine.CharacterMovementComponent|GetMaxWalkSpeed (Variables|Character|GetCharacterMovement)) 0.5)
    (Variables|PlayerMovement|SetIsMoving true)
    (Utilities|FlowControl|Sequence
      (:then_0
        (bind _outhit (Collision|LineTraceForObjects _returnvalue (+ (- _returnvalue "0.000000,0.000000,100.000000") (* (Variables|PlayerMovement|GetMoveDirection) (Math|Vector|MakeVector _stopdistance _stopdistance 0.0))) (Utilities|Array|MakeArray "ObjectTypeQuery4" "ObjectTypeQuery3") false 0 "ForOneFrame"))
        (if (.bBlockingHit (Collision|BreakHitResult _outhit))
          (Variables|PlayerMovement|SetIsMoving false)
          (Variables|PlayerMovement|SetCanChangeDirection true)
          (return)
          (else
            (Pawn|Input|AddMovementInput (Variables|PlayerMovement|GetMoveDirection) 1.0 false)
            (return)))))
    (else
      (Variables|PlayerMovement|SetIsMoving false)
      (Variables|PlayerMovement|SetCanChangeDirection true))))

(fn FPlayerTakeDamage
  (params (TakeDamage :type Float%20%28single-precision%29))
  (if (not (Variables|Default|GetisPlayerDead?))
    (if (== (Variables|Default|GetTempLives) 1)
      (bind _output_get (Variables|Default|SetTempLives (Math|Float|Truncate (- (Variables|Default|GetTempLives) (Variables|Default|GetDamageTakenValue)))))
      (Development|PrintText (Utilities|Text|FormatText "Player Temp Lives: {count}" _output_get))
      (return)
      (else
        (bind _output_get_2 (Variables|Default|SetBasePlayerLives (Math|Float|Truncate (- (Variables|Default|GetBasePlayerLives) (Variables|Default|GetDamageTakenValue)))))
        (Development|PrintText (Utilities|Text|FormatText "Player Health: {count}" _output_get_2))
        (CallFunction|FSetPLayerHealth)
        (if (and (<= (Variables|Default|GetBasePlayerLives) 0) (<= (Variables|Default|GetTempLives) 0))
          (if (not (Variables|Default|GetisPlayerDead?))
            (CallFunction|PlayerIsDead)
            (CallFunction|FPlayersDeath)
            (bind _asbp_ya_game_mode (Utilities|Casting|CastToBP_YA_GameMode (Game|GetGameMode)))
            (Default|FPlayerLose _asbp_ya_game_mode)
            (Development|PrintString "You are Dead")
            (return)))))))

(fn FRemoveTempLivesTimer
  (params (DeltaSeconds :type Float%20%28double-precision%29))
  (if (> (Variables|Default|GetTempLiveTiimer) 0.0)
    (Variables|Default|SetTempLiveTiimer (Variables|Default|GetTempLiveTiimer))
    (bind _output_get (Variables|Default|SetTempLiveTiimer (- (Variables|Default|GetTempLiveTiimer) DeltaSeconds)))
    (if (<= _output_get 0.0)
      (Variables|Default|SetTempLives (- (Variables|Default|GetTempLives) 1))
      (return))))

(fn FInteractionLineTrace
  (bind _returnvalue (Transformation|GetActorLocation))
  (bind _outhit (Collision|LineTraceByChannel _returnvalue (+ _returnvalue (* (Transformation|GetActorForwardVector) 1.5e+02)) "TraceTypeQuery1" false 0 "ForOneFrame"))
  (if (.bBlockingHit (Collision|BreakHitResult _outhit))
    (if (Utilities|DoesObjectImplementInterface (.HitActor (Collision|BreakHitResult _outhit)) "/Game/_Main/Interfaces/BP_InteractInterface.BP_InteractInterface_C")
      (Variables|Default|SetHit%20Actor (.HitActor (Collision|BreakHitResult _outhit)))
      (return)
      (else
        _)))
  (Variables|Default|SetHit%20Actor 0)
  (return))

(fn FSpawnBombAbilitie
  (bind _returnvalue (Game|SpawnActorfromClass "/Game/_Main/Blueprints/Bomb/BP_Bomb.BP_Bomb_C" (Math|Transform|MakeTransform (+ (Transformation|GetActorLocation) (* (Transformation|GetActorForwardVector) "-100.000000,-100.000000,0.000000")) (Transformation|GetActorRotation)) "AlwaysSpawn" "MultiplyWithRoot" 0 0))
  (Physics|AddImpulse (Variables|/Game/_Main/Blueprints/Bomb/BP_Bomb.BP_Bomb_C|GetSM_Stone01 _returnvalue) (* (Transformation|GetActorForwardVector) "1000.000000,1000.000000,1000.000000") "None" false)
  (Development|PrintString "You create a Bomb")
  (return))

(fn FAbilitieOneTimer
  (params (DeltaSeconds :type Float%20%28double-precision%29))
  (if (Variables|Default|GetisAbilitieTimerActive?)
    (bind _output_get (Variables|Default|SetAbilitieCooldownTimer (- (Variables|Default|GetAbilitieCooldownTimer) DeltaSeconds)))
    (if (<= _output_get 0.0)
      (Widget|SetVisibility (Variables|/Game/_Main/UI_Widgets/WBP_BombAbilitie.WBP_BombAbilitie_C|GetAbilitieTimerText (Variables|/Game/_Main/UI_Widgets/WBP_MainHUD.WBP_MainHUD_C|GetWBP_BombAbilitie (Variables|Default|GetMainHUDRef))) "Hidden")
      (Variables|Default|SetisAbilitieTimerActive? false)
      (Variables|Default|SetCanSpawnBomb true)
      (Variables|Default|SetAbilitieCooldownTimer (Variables|Default|GetSetedAbilitieCooldownTimer))
      (return))))

(fn PickUpItems
  (return "" false))