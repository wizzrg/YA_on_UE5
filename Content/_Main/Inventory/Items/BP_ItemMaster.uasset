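; Base world item actor for the inventory system, representing an item that can be picked up.
; The construction script reads a data table row, either the configured one or a random Wood or Stone pick, caches it as CraftItem and applies its static mesh.
; PickUpItems hands CraftItem to the caller and always allows pickup.
; Interact and cursor events are empty; the hover info widget and debug trace print are left unwired.
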(event `self.ReceiveBeginPlay`)

(event `self.ReceiveActorBeginCursorOver`)

(event `self.ReceiveActorEndCursorOver`)

(event `/Game/_Main/Interfaces/BP_InteractInterface.Interact`)

(fn `OnMouseHoverStart`
  (`KismetSystemLibrary.PrintString` (`KismetSystemLibrary.GetDisplayName` (`.HitActor` (`GameplayStatics.BreakHitResult` (`PlayerController.GetHitResultUnderCursorByChannel` (`GameplayStatics.GetPlayerController` 0) "TraceTypeQuery1" true)))))
  (return))

(fn `PickUpItems`
  (returns (ItemCraft :type "/Game/_Main/InventoryAndCrafting/S_CraftItemMaster Structure") (`CanPickup?` :type Boolean))
  (return (`self.CraftItem`) true))

(fn `UserConstructionScript`
  (bind (_itemdatarow_datatable _itemdatarow_rowname) (break `DataTableRowHandle` (`self.ItemDataRow`)))
  (if (not (`self.random Item?`))
    (bind _returnvalue (`|GetDataTableRow` _itemdatarow_datatable _itemdatarow_rowname)
      (:`then`
        (set `self.CraftItem` _returnvalue)))
    (else
      (bind _returnvalue_2 (`|GetDataTableRow` _itemdatarow_datatable (`KismetArrayLibrary.Array_Random` (`|MakeArray` "Wood" "Stone" :!type "Name")))
        (:`then`
          (set `self.CraftItem` _returnvalue_2)))))
  (`StaticMeshComponent.SetStaticMesh` (`self.ItemMesh`) (`.StaticMesh_9_F14BFC304909F7A8601BBCBC025840C7` (break `/Game/_Main/InventoryAndCrafting/S_CraftItemMaster` (`self.CraftItem`)))))