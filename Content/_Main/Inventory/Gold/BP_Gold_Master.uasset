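; Base gold pickup actor whose mesh and value come from a row in DT_Gold, selected by its Gold row handle's row name.
; The construction script sets GoldMesh from that row.
; When BP_Player overlaps the Sphere, it adds the row's Amount to GoldCount in BP_YA_GameInstance, destroys itself and prints a "Gold Added" message.
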(event `self.Sphere.OnComponentBeginOverlap`
  (params (OverlappedComponent :type "PrimitiveComponent Object Reference") (OtherActor :type "Actor Object Reference") (OtherComp :type "PrimitiveComponent Object Reference") (OtherBodyIndex :type Integer) (bFromSweep :type Boolean) (SweepResult :type "HitResult Structure (by ref)"))
  (bind _asbp_player (cast `/Game/_Main/Player/BP_Player` OtherActor))
  (`/Engine/EditorBlueprintResources/StandardMacros.IsValid` _asbp_player
    (:`Is Valid`
      (bind _returnvalue (`|GetDataTableRow` "/Game/_Main/Inventory/DataTables/DT_Gold.DT_Gold" (`.RowName` (break `DataTableRowHandle` (`self.Gold`))))
        (:`then`
          (bind _asbp_ya_game_instance (cast `/Game/_Main/Blueprints/BP_YA_GameInstance` (`GameplayStatics.GetGameInstance`)))
          (set `/Game/_Main/Blueprints/BP_YA_GameInstance.GoldCount` (+ (`.Amount_7_ADD076E24F078873E83B2A9E5001BBBF` (break `/Game/_Main/Blueprints/Structures/S_Gold` _returnvalue)) (`/Game/_Main/Blueprints/BP_YA_GameInstance.GoldCount` _asbp_ya_game_instance)) _asbp_ya_game_instance)
          (`self.K2_DestroyActor`)
          (`KismetSystemLibrary.PrintString` "Gold Added" true true (struct :`R` 0.23018 :`G` 1.0 :`A` 1.0)))))))

(fn `UserConstructionScript`
  (bind (_gold_datatable _gold_rowname) (break `DataTableRowHandle` (`self.Gold`)))
  (bind _returnvalue (`|GetDataTableRow` "/Game/_Main/Inventory/DataTables/DT_Gold.DT_Gold" _gold_rowname)
    (:`then`
      (`StaticMeshComponent.SetStaticMesh` (`self.GoldMesh`) (`.Mesh_8_939D712F4E0688AECC2BD4975B64B048` (break `/Game/_Main/Blueprints/Structures/S_Gold` _returnvalue))))))