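; Base artefact pickup that bobs vertically in the world and adds to the player's artefact count when collected.
; The construction script sets its mesh from the selected DT_Artefact row.
; Overlapping the sphere with BP_Player adds that row's Amount to ArtefactCount in the game instance, destroys the actor and prints a confirmation.
; Tick drives the bob with a sine-based world offset applied each frame, unscaled by delta time.
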(event `self.ReceiveTick`
  (params (DeltaSeconds :type "Float (single-precision)"))
  (bind _output_get (set `self.TimeRunning` (+ DeltaSeconds (`self.TimeRunning`))))
  (bind _returnvalue (`KismetMathLibrary.Sin` (* _output_get 3.0)))
  (`self.K2_AddActorWorldOffset` (`KismetMathLibrary.MakeVector` 0.0 0.0 (`KismetMathLibrary.Lerp` _returnvalue (* _returnvalue 5.0)))))

(event `self.Sphere.OnComponentBeginOverlap`
  (params (OverlappedComponent :type "PrimitiveComponent Object Reference") (OtherActor :type "Actor Object Reference") (OtherComp :type "PrimitiveComponent Object Reference") (OtherBodyIndex :type Integer) (bFromSweep :type Boolean) (SweepResult :type "HitResult Structure (by ref)"))
  (bind _asbp_player (cast `/Game/_Main/Player/BP_Player` OtherActor))
  (`/Engine/EditorBlueprintResources/StandardMacros.IsValid` _asbp_player
    (:`Is Valid`
      (bind _returnvalue (`|GetDataTableRow` "/Game/_Main/Inventory/DataTables/DT_Artefact.DT_Artefact" (`.RowName` (break `DataTableRowHandle` (`self.ArtefactDT`))))
        (:`then`
          (bind _asbp_ya_game_instance (cast `/Game/_Main/Blueprints/BP_YA_GameInstance` (`GameplayStatics.GetGameInstance`)))
          (set `/Game/_Main/Blueprints/BP_YA_GameInstance.ArtefactCount` (+ (`.Amount_7_5BF8295A4E62C94C988F198E46C365D6` (break `/Game/_Main/Blueprints/Structures/S_Artefacts` _returnvalue)) (`/Game/_Main/Blueprints/BP_YA_GameInstance.ArtefactCount` _asbp_ya_game_instance)) _asbp_ya_game_instance)
          (`self.K2_DestroyActor`)
          (`KismetSystemLibrary.PrintString` "Artefact Added" true true (struct :`G` 0.424858 :`B` 1.0 :`A` 1.0)))))))

(fn `UserConstructionScript`
  (bind (_artefactdt_datatable _artefactdt_rowname) (break `DataTableRowHandle` (`self.ArtefactDT`)))
  (bind _returnvalue (`|GetDataTableRow` "/Game/_Main/Inventory/DataTables/DT_Artefact.DT_Artefact" _artefactdt_rowname)
    (:`then`
      (`StaticMeshComponent.SetStaticMesh` (`self.ArtefactMesh`) (`.StaticMesh_8_FF4C55094A618876C47FEBB329501C8D` (break `/Game/_Main/Blueprints/Structures/S_Artefacts` _returnvalue))))))