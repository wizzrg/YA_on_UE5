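; Player inventory and crafting component that manages item pickup, the item array and the inventory screen.
; Each tick, a sphere trace finds BP_ItemMaster pickups for the interact prompt, while a line trace caches BPI_MyInteract actors.
; Interact plays a running or standing montage, stacks the item by name and notifies the HUD; other interactables only print a crafting-table message.
; CanCraft checks DataTable-referenced ingredients against held amounts, and RemoveItem decrements or deletes stacks.
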(event `self.ReceiveBeginPlay`
  (bind _asbp_player (cast `/Game/_Main/Player/BP_Player` (`GameplayStatics.GetPlayerCharacter` 0)))
  (set `self.PlayerRef` _asbp_player)
  (bind _returnvalue (`|CreateWidget` "/Game/_Main/InventoryAndCrafting/WB_InventoryAndCrafting.WB_InventoryAndCrafting_C"))
  (set `self.InventoryWidgetRef` _returnvalue)
  (bind _returnvalue_2 (`|CreateWidget` "/Game/_Main/UI_Widgets/WBP_Interact.WBP_Interact_C"))
  (set `self.InteractWidgetRef` _returnvalue_2))

(event `EnhancedInput|/Game/TopDown/Input/Actions/IA_Inventory`
  (params (ActionValue :type Boolean) (ElapsedSeconds :type "Float (double-precision)") (TriggeredSeconds :type "Float (double-precision)") (InputAction :type "InputAction Object Reference" :default "/Game/TopDown/Input/Actions/IA_Inventory.IA_Inventory"))
  (bind _returnvalue (`GameplayStatics.GetPlayerController` 0))
  (bind _returnvalue_2 (`GameplayStatics.GetPlayerController` 0))
  (bind _inventorywidgetref (`self.InventoryWidgetRef`))
  (bind _inventorywidgetref_2 (`self.InventoryWidgetRef`))
  (:`Started`
    (`self.InventoryWidgetRef`
      (:`then`
        (bind _returnvalue_3 (`|CreateWidget` "/Game/_Main/InventoryAndCrafting/WB_InventoryAndCrafting.WB_InventoryAndCrafting_C"))
        (bind _output_get (set `self.InventoryWidgetRef` _returnvalue_3))
        (`UserWidget.AddToViewport` _output_get 0)
        (set `PlayerController.bShowMouseCursor` true _returnvalue)
        (`WidgetBlueprintLibrary.SetInputMode_UIOnlyEx` _returnvalue _inventorywidgetref)
        (`/Game/_Main/InventoryAndCrafting/WB_InventoryAndCrafting.UpdateNewInventory` _inventorywidgetref))
      (:`else`
        (`Widget.RemoveFromParent` _inventorywidgetref_2 :!label _label)
        (set `self.InventoryWidgetRef` _inventorywidgetref_2)
        (set `PlayerController.bShowMouseCursor` true _returnvalue_2)
        (`WidgetBlueprintLibrary.SetInputMode_GameOnly` _returnvalue_2)))))

(event `CloseInventory`
  (goto _label))

(event `self.ReceiveTick`
  (params (DeltaSeconds :type "Float (single-precision)"))
  (bind _interactwidgetref (`self.InteractWidgetRef`))
  (`self.InteractingLineTrace`)
  (bind (_item _founditem_) (`self.TraceItemToPickUp`))
  (set `/Game/_Main/UI_Widgets/WBP_Interact.ItemFind` _item (`self.InteractWidgetRef`))
  (if _founditem_
    (`UserWidget.AddToViewport` _interactwidgetref 0)
    (else
      (`Widget.RemoveFromParent` _interactwidgetref))))

(event `EnhancedInput|/Game/TopDown/Input/Actions/IA_Interact`
  (params (ActionValue :type Boolean) (ElapsedSeconds :type "Float (double-precision)") (TriggeredSeconds :type "Float (double-precision)") (InputAction :type "InputAction Object Reference" :default "/Game/TopDown/Input/Actions/IA_Interact.IA_Interact"))
  (bind _playerref (`self.PlayerRef`))
  (bind _mesh (`Character.Mesh` _playerref))
  (:`Started`
    (`|ExecutionSequence`
      (:`then_0`
        (bind (_item _founditem_ _itemactor) (`self.TraceItemToPickUp`))
        (if _founditem_
          (if (> (`KismetMathLibrary.VSize` (`MovementComponent.Velocity` (`Character.CharacterMovement` _playerref))) 0.0)
            (`|PlayMontage` _mesh "/Game/_Main/Player/YA_Character/Adam_Char/Animations/AM_RunPickup.AM_RunPickup"
              (:`then`
                _))
            (else
              (`|PlayMontage` _mesh "/Game/_Main/Player/YA_Character/Adam_Char/Animations/AM_StandPickUpItem.AM_StandPickUpItem"
                (:`then`
                  _))))
          (`self.AddItem` _item)
          (`Actor.K2_DestroyActor` _itemactor)
          (else
            (`self.Hit Actor`
              (:`then`
                (`KismetSystemLibrary.PrintString` "Crafting Table Open" true true (struct :`R` 0.901533 :`G` 1.0 :`A` 1.0)))
              (:`else`))))))))

(fn `AddItem`
  (params (NewItem :type "/Game/_Main/InventoryAndCrafting/S_CraftItemMaster Structure"))
  (locals (`ExistingItem?` :type Boolean))
  (bind (_name _amount _staticmesh _icon) (break `/Game/_Main/InventoryAndCrafting/S_CraftItemMaster` (`local.NewItem`)))
  (bind (_name_2 _amount_2 _staticmesh_2 _icon_2 _cancraft_ _resourcesneeded _addhealth _equipedactor) (break `/Game/_Main/InventoryAndCrafting/S_CraftItemMaster` (`local.NewItem`)))
  (for (_array_element _array_index) (`self.Items`)
    (bind (_name_3 _amount_3) (break `/Game/_Main/InventoryAndCrafting/S_CraftItemMaster` _array_element))
    (if (`KismetStringLibrary.EqualEqual_StrStr` _name_3 _name_2)
      ;[1 1 1] Stack Items
      (`KismetArrayLibrary.Array_Set` (`self.Items`) _array_index (make `/Game/_Main/InventoryAndCrafting/S_CraftItemMaster` _name_2 (+ _amount_3 _amount_2) _staticmesh_2 _icon_2 _cancraft_ _resourcesneeded _addhealth _equipedactor))
      (set `local.ExistingItem?` true)
      (break)))
  ;[1 1 1] Item Notification Anim
  (bind _mainhudref (`/Game/_Main/Player/BP_Player.MainHUDRef` (`self.PlayerRef`))
    (:`then`
      (`/Game/_Main/UI_Widgets/WBP_MainHUD.Add Item Notification` _mainhudref _name _icon _amount)
      ;[1 1 1] New Item
      (if (not (`local.ExistingItem?`))
        (`KismetArrayLibrary.Array_Add` (`self.Items`) (`local.NewItem`))))
    (:`else`)))

(fn `CanCraft`
  (params (Item :type "/Game/_Main/InventoryAndCrafting/S_CraftItemMaster Structure"))
  (returns (`CanCraft?` :type Boolean))
  (locals (LocalCraftingTotalAmount :type Integer))
  (bind (_name _amount _staticmesh _icon _cancraft_ _resourcesneeded) (break `/Game/_Main/InventoryAndCrafting/S_CraftItemMaster` Item))
  (for _array_element _resourcesneeded
    (bind (_item _amount_2) (break `/Game/_Main/InventoryAndCrafting/S_CraftingRecipe` _array_element))
    (bind (_datatable _rowname) (break `DataTableRowHandle` _item))
    (bind _returnvalue (`|GetDataTableRow` _datatable _rowname)
      (:`then`
        (for _array_element_2 (`self.Items`)
          (bind (_name_2 _amount_3) (break `/Game/_Main/InventoryAndCrafting/S_CraftItemMaster` _array_element_2))
          (if (and (`KismetStringLibrary.EqualEqual_StrStr` (`.Name_5_2BD976C147DF416139DA2A84BA3D98AC` (break `/Game/_Main/InventoryAndCrafting/S_CraftItemMaster` _returnvalue)) _name_2) (>= _amount_3 _amount_2))
            (`/Engine/EditorBlueprintResources/StandardMacros.IncrementInt` (`local.LocalCraftingTotalAmount`)
              (:`  `
                (break))))))))
  (if (>= (`local.LocalCraftingTotalAmount`) (`KismetArrayLibrary.Array_Length` _resourcesneeded))
    (return true)
    (else
      (return false))))

(fn `InteractingLineTrace`
  (bind _returnvalue (`GameplayStatics.GetPlayerCharacter` 0))
  (bind _returnvalue_2 (`Actor.K2_GetActorLocation` _returnvalue))
  (bind _outhit (`KismetSystemLibrary.LineTraceSingle` :`Start` _returnvalue_2 :`End` (+ _returnvalue_2 (* (`Actor.GetActorForwardVector` _returnvalue) 150.0)) :`TraceChannel` "TraceTypeQuery1" :`DrawDebugType` "ForOneFrame"))
  (bind (_bblockinghit _binitialoverlap _time _distance _location _impactpoint _normal _impactnormal _physmat _hitactor) (`GameplayStatics.BreakHitResult` _outhit))
  (if _bblockinghit
    (if (`KismetSystemLibrary.DoesImplementInterface` _hitactor "/Game/_Main/Interfaces/BPI_MyInteract.BPI_MyInteract_C")
      (set `self.Hit Actor` _hitactor)
      (return)
      (else
        _)))
  (set `self.Hit Actor` null)
  (return))

(fn `RemoveItem`
  (params (Item :type "/Game/_Main/InventoryAndCrafting/S_CraftItemMaster Structure") (`DecreaseOneOnly?` :type Boolean))
  (returns (`NoMoreLeft?` :type Boolean))
  (bind (_name _amount) (break `/Game/_Main/InventoryAndCrafting/S_CraftItemMaster` (`local.Item`)))
  (bind (_name_2 _amount_2 _staticmesh _icon _cancraft_ _resourcesneeded _addhealth _equipedactor) (break `/Game/_Main/InventoryAndCrafting/S_CraftItemMaster` (`local.Item`)))
  (for (_array_element _array_index) (`self.Items`)
    (bind (_name_3 _amount_3) (break `/Game/_Main/InventoryAndCrafting/S_CraftItemMaster` _array_element))
    (if (`KismetStringLibrary.EqualEqual_StrStr` _name_3 _name)
      (if (< _amount_3 2)
        (`KismetArrayLibrary.Array_Remove` (`self.Items`) _array_index :!label _label)
        (`|ExecutionSequence`
          (:`then_0`
            (break))
          (:`then_1`
            (return true)))
        (else
          (bind _returnvalue (- _amount_3 (`KismetMathLibrary.SelectInt` 1 _amount (`local.DecreaseOneOnly?`))))
          (if (> _returnvalue 0)
            (`KismetArrayLibrary.Array_Set` (`self.Items`) _array_index (make `/Game/_Main/InventoryAndCrafting/S_CraftItemMaster` _name_2 _returnvalue _staticmesh _icon _cancraft_ _resourcesneeded _addhealth _equipedactor))
            (else
              (goto _label))))))))

(fn `TraceItemToPickUp`
  (returns (Item :type "/Game/_Main/InventoryAndCrafting/S_CraftItemMaster Structure") (`FoundItem?` :type Boolean) (ItemActor :type "Actor Object Reference"))
  (bind _returnvalue (`GameplayStatics.GetPlayerCharacter` 0))
  (bind _returnvalue_2 (- (`Actor.K2_GetActorLocation` _returnvalue) (0.0 0.0 0.0)))
  (bind _outhit (`KismetSystemLibrary.SphereTraceSingle` :`Start` _returnvalue_2 :`End` (+ _returnvalue_2 (* (`Actor.GetActorForwardVector` _returnvalue) 225.0)) :`Radius` 90.0 :`TraceChannel` "TraceTypeQuery1" :`DrawDebugType` "ForOneFrame"))
  (bind (_bblockinghit _binitialoverlap _time _distance _location _impactpoint _normal _impactnormal _physmat _hitactor) (`GameplayStatics.BreakHitResult` _outhit))
  (bind _asbp_item_master (cast `/Game/_Main/Inventory/Items/BP_ItemMaster` _hitactor)
    (:`then`
      (bind _output_get (set `self.ItemCraftMaster` _asbp_item_master))
      (`/Engine/EditorBlueprintResources/StandardMacros.IsValid` _output_get
        (:`Is Valid`
          (return (`/Game/_Main/Inventory/Items/BP_ItemMaster.CraftItem` _asbp_item_master) true _hitactor))))
    (:`CastFailed`
      (return (struct) false null))))