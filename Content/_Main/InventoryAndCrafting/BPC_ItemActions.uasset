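; Player component that carries out the action of the currently equipped inventory item when the attack input fires.
; BeginPlay caches player and inventory references, then IA_Attack switches on the item name.
; The pickaxe plays a montage whose notify sphere-traces ahead to apply damage, with re-use locked until it ends.
; Consumables are removed through the inventory, then clear the equipped item and add a life or set walk speed without resetting it.
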(event `self.ReceiveBeginPlay`
  ;[1 1 1] Initialize Variables
  (bind _asbp_player (cast `/Game/_Main/Player/BP_Player` (`self.GetOwner`)))
  (`/Engine/EditorBlueprintResources/StandardMacros.IsValid` _asbp_player
    (:`Is Valid`
      (bind _output_get (set `self.PlayerRef` _asbp_player))
      (bind _output_get_2 (set `self.Inventory and CraftingRef` (`/Game/_Main/Player/BP_Player.AC_InventoryAndCrafting` _output_get)))
      (set `self.Inventory Widget Ref` (`/Game/_Main/InventoryAndCrafting/AC_InventoryAndCrafting.InventoryWidgetRef` _output_get_2)))))

(event `AttackAndHarvest`
  (bind _returnvalue (`GameplayStatics.GetPlayerCharacter` 0))
  (bind _returnvalue_2 (`Actor.K2_GetActorLocation` _returnvalue))
  (if (`self.CanAttack?`)
    (`|PlayMontage` (`Character.Mesh` (`self.PlayerRef`)) "/Game/_Main/Player/YA_Character/Adam_Char/Animations/AM_Attack.AM_Attack"
      (:`then`
        (set `self.CanAttack?` false))
      (:`OnCompleted`
        (set `self.CanAttack?` true :!label _label))
      (:`OnInterrupted`
        (goto _label))
      (:`OnNotifyBegin`
        (bind (_outhit _returnvalue_3) (`KismetSystemLibrary.SphereTraceSingleForObjects` _returnvalue_2 (+ _returnvalue_2 (* (`Actor.GetActorForwardVector` _returnvalue) 150.0)) 25.0 (`|MakeArray` "ObjectTypeQuery2" "ObjectTypeQuery1" "ObjectTypeQuery3" :!type "EObjectTypeQuery Enum") false (`|MakeArray` (`self.GetOwner`)) "ForDuration"))
        (if _returnvalue_3
          (`GameplayStatics.ApplyDamage` (`.HitActor` (`GameplayStatics.BreakHitResult` _outhit)) 10.0 null (`self.GetOwner`)))))))

(event `EnhancedInput|/Game/TopDown/Input/Actions/IA_Interact`
  (params (ActionValue :type Boolean) (ElapsedSeconds :type "Float (double-precision)") (TriggeredSeconds :type "Float (double-precision)") (InputAction :type "InputAction Object Reference" :default "/Game/TopDown/Input/Actions/IA_Interact.IA_Interact")))

(event `EnhancedInput|/Game/TopDown/Input/Actions/IA_Attack`
  (params (ActionValue :type Boolean) (ElapsedSeconds :type "Float (double-precision)") (TriggeredSeconds :type "Float (double-precision)") (InputAction :type "InputAction Object Reference" :default "/Game/TopDown/Input/Actions/IA_Attack.IA_Attack"))
  (:`Triggered`
    (switch `string` (`.Name_5_2BD976C147DF416139DA2A84BA3D98AC` (break `/Game/_Main/InventoryAndCrafting/S_CraftItemMaster` (`/Game/_Main/InventoryAndCrafting/AC_InventoryAndCrafting.EquipedItem` (`self.Inventory and CraftingRef`))))
      (:`Apple`
        (`self.Eat` :!label _label_2))
      (:`Apple Pie`
        (goto _label_2))
      (:`Healing Potion`
        (goto _label_2))
      (:`Pickaxe`
        (`self.AttackAndHarvest`))
      (:`Speed Potion`
        (`self.EatSpeedPotion`)))))

(event `Eat`
  (bind _playerref (`self.PlayerRef`))
  (bind _playerref_2 (`self.PlayerRef`))
  (bind _inventory_and_craftingref (`self.Inventory and CraftingRef`))
  (`/Engine/EditorBlueprintResources/StandardMacros.IsValid` _playerref_2
    (:`Is Valid`
      (if (< (`/Game/_Main/Player/BP_Player.BasePlayerLives` _playerref_2) (`/Game/_Main/Player/BP_Player.BaseMaxPlayerLives` _playerref_2))
        (`GameplayStatics.PlaySound2D` "/Game/GatheringResourcesSystem/Sounds/Sound_CrystalHit.Sound_CrystalHit" 1.0 1.0 0.0 null null)
        (bind _nomoreleft_ (`/Game/_Main/InventoryAndCrafting/AC_InventoryAndCrafting.RemoveItem` _inventory_and_craftingref (`/Game/_Main/InventoryAndCrafting/AC_InventoryAndCrafting.EquipedItem` _inventory_and_craftingref) true))
        (if _nomoreleft_
          (bind _output_get (set `/Game/_Main/InventoryAndCrafting/AC_InventoryAndCrafting.EquipedItem` (struct) (`self.Inventory and CraftingRef`)))
          (`/Game/_Main/Player/BP_Player.EquipedItemMesh` (`self.PlayerRef`) _output_get)
          (`/Engine/EditorBlueprintResources/StandardMacros.IsValid` _playerref
            (:`Is Valid`
              (set `/Game/_Main/Player/BP_Player.BasePlayerLives` (`KismetMathLibrary.Clamp` (+ (`/Game/_Main/Player/BP_Player.BasePlayerLives` _playerref) 1) 0 (`/Game/_Main/Player/BP_Player.BaseMaxPlayerLives` _playerref)) _playerref)
              (`KismetSystemLibrary.PrintText` (`|FormatText` "You eat and add: {health}" _)))))
        (else
          (`KismetSystemLibrary.PrintString` "Lives is Full"))))))

(event `EatSpeedPotion`
  (bind _inventory_and_craftingref (`self.Inventory and CraftingRef`))
  (`/Engine/EditorBlueprintResources/StandardMacros.IsValid` (`self.PlayerRef`)
    (:`Is Valid`
      (`GameplayStatics.PlaySound2D` "/Engine/EditorSounds/Notifications/CompileFailed.CompileFailed" 1.0 1.0 0.0 null null)
      (bind _nomoreleft_ (`/Game/_Main/InventoryAndCrafting/AC_InventoryAndCrafting.RemoveItem` _inventory_and_craftingref (`/Game/_Main/InventoryAndCrafting/AC_InventoryAndCrafting.EquipedItem` _inventory_and_craftingref) true))
      (if _nomoreleft_
        (bind _output_get (set `/Game/_Main/InventoryAndCrafting/AC_InventoryAndCrafting.EquipedItem` (struct) (`self.Inventory and CraftingRef`)))
        (`/Game/_Main/Player/BP_Player.EquipedItemMesh` (`self.PlayerRef`) _output_get)
        (set `CharacterMovementComponent.MaxWalkSpeed` 400.0 (`Character.CharacterMovement` (`self.PlayerRef`)))))))