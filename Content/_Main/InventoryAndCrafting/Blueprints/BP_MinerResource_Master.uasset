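; BP_MinerResource_Master is a harvestable resource node, apparently a base for minable resources, that yields craft items when damaged.
; AnyDamage only reacts to damage causers implementing the BP_Inventory interface, subtracting Health and destroying the node at zero.
; Each non-lethal hit picks a random Items entry, looks it up in DT_CraftItems and sends it to the causer via HarvestItem with a randomized amount.
; The final, destroying hit yields nothing.
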(event `self.ReceiveAnyDamage`
  (params (Damage :type "Float (single-precision)") (DamageType :type "DamageType Object Reference") (InstigatedBy :type "Controller Object Reference") (DamageCauser :type "Actor Object Reference"))
  (if (`KismetSystemLibrary.DoesImplementInterface` DamageCauser "/Game/_Main/Interfaces/BP_Inventory.BP_Inventory_C")
    (bind _output_get (set `self.Health` (- (`self.Health`) Damage)))
    (if (<= _output_get 0.0)
      (`self.K2_DestroyActor`)
      (else
        (bind _returnvalue (`|GetDataTableRow` "/Game/_Main/InventoryAndCrafting/DT_CraftItems.DT_CraftItems" (`.RowName` (break `DataTableRowHandle` (`KismetArrayLibrary.Array_Random` (`self.Items`)))))
          (:`then`
            (bind (_name _amount _staticmesh _icon _cancraft_ _resourcesneeded _addhaelth) (break `/Game/_Main/InventoryAndCrafting/S_CraftItemMaster` _returnvalue))
            (message `/Game/_Main/Interfaces/BP_Inventory.HarvestItem` DamageCauser (make `/Game/_Main/InventoryAndCrafting/S_CraftItemMaster` _name (`KismetMathLibrary.RandomIntegerInRange` _amount 5) _staticmesh _icon _cancraft_ _resourcesneeded _addhaelth))))))))

(event `/Game/_Main/Interfaces/BP_Inventory.HarvestItem`
  (params (Item :type "/Game/_Main/InventoryAndCrafting/S_CraftItemMaster Structure")))

(fn `UserConstructionScript`)